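; BP_DoorWithPressureSwitch is a door, named for pressure switch use, that animates open and closed.
; OpenDoor plays DoorTimeline and CloseDoor reverses it, with each update feeding UpdateDoorLocation to move the door.
; The timeline's Finished output toggles IsDoorOpen.
; No switch trigger logic appears in these graphs; a debug print of SwitchHandle's remaining timer is left disconnected.
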(event `self.OpenDoor`
  ;[1 1 1] Close/Open Door
  (bind (_direction _float) (`Timeline|DoorTimeline` :!label _label)
    (:`Update`
      (`self.UpdateDoorLocation` _float))
    (:`Finished`
      (if (`self.bIsDoorOpen`)
        (set `self.bIsDoorOpen` false)
        (else
          (set `self.bIsDoorOpen` true))))))

(event `self.CloseDoor`
  ;[1 1 1] Close/Open Door
  (goto _label :!via `Reverse`))

(event `self.ReceiveTick`
  (params (DeltaSeconds :type "Float (single-precision)"))
  ;[1 1 1] Tick
)

(fn `UserConstructionScript`)