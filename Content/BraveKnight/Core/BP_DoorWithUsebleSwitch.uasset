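; Timed door Blueprint that slides open on OpenDoor and closes itself after SwitchTime, presumably triggered by a usable switch.
; A single timeline drives UpdateDoorLocation, playing forward to open and reversing to close.
; Its Finished output toggles IsDoorOpen, starting the auto-close timer once open and clearing it once closed.
; CloseDoor reverses the timeline directly, and a disconnected debug print of remaining time never runs.
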(event `self.OpenDoor`
  ;[1 1 1] Close/Open Door
  (bind (_direction _float) (`Timeline|CloseOpenTimeline` :!label _label)
    (:`Update`
      (`self.UpdateDoorLocation` _float))
    (:`Finished`
      (if (`self.bIsDoorOpen`)
        (set `self.bIsDoorOpen` false)
        (`KismetSystemLibrary.K2_ClearAndInvalidateTimerHandle` (`self.SwitchHandle`))
        (else
          (set `self.bIsDoorOpen` true)
          (bind _returnvalue (`KismetSystemLibrary.K2_SetTimerDelegate` (delegate `CloseDoorCall`) (`self.SwitchTime`)))
          (set `self.SwitchHandle` _returnvalue))))))

(event `self.CloseDoor`
  ;[1 1 1] Close/Open Door
  (goto _label :!via `Reverse`))

(event `CloseDoorCall`
  ;[1 1 1] Close/Open Door
  (goto _label :!via `Reverse`))

(event `self.ReceiveTick`
  (params (DeltaSeconds :type "Float (single-precision)"))
  ;[1 1 1] Tick
)

(fn `UserConstructionScript`)