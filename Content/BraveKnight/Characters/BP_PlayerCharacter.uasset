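; Player character Blueprint for BraveKnight that handles object interaction and creates the player's HUD.
; Capsule overlaps maintain an array of nearby UsebleObjects, and the Use input calls UseObject on each of them.
; BeginPlay builds the main canvas widget, then inserts health and stamina bar widgets into its containers, giving each a reference to the character.
; Tick calls the parent and prints Stamina on screen.
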(event `self.CapsuleComponent.OnComponentEndOverlap`
  (params (OverlappedComponent :type "PrimitiveComponent Object Reference") (OtherActor :type "Actor Object Reference") (OtherComp :type "PrimitiveComponent Object Reference") (OtherBodyIndex :type Integer))
  (bind _overlappdedusebleobjects (`self.OverlappdedUsebleObjects`))
  (bind _asuseble_object (cast `UsebleObject` OtherActor))
  (bind _returnvalue (`KismetArrayLibrary.Array_Find` _overlappdedusebleobjects _asuseble_object))
  (if (`KismetArrayLibrary.Array_IsValidIndex` _overlappdedusebleobjects _returnvalue)
    (`KismetArrayLibrary.Array_Remove` _overlappdedusebleobjects _returnvalue)))

(event `self.CapsuleComponent.OnComponentBeginOverlap`
  (params (OverlappedComponent :type "PrimitiveComponent Object Reference") (OtherActor :type "Actor Object Reference") (OtherComp :type "PrimitiveComponent Object Reference") (OtherBodyIndex :type Integer) (bFromSweep :type Boolean) (SweepResult :type "HitResult Structure (by ref)"))
  (bind _asuseble_object (cast `UsebleObject` OtherActor))
  (`KismetArrayLibrary.Array_AddUnique` (`self.OverlappdedUsebleObjects`) _asuseble_object))

(event `InputAction|Use`
  (params (Key :type "Key Structure"))
  (:`Pressed`
    (for _array_element (`self.OverlappdedUsebleObjects`)
      (bind _asuseble_object (cast `UsebleObject` _array_element))
      (`UsebleObject.UseObject` _asuseble_object))))

(event `self.ReceiveBeginPlay`
  (bind _maincanvas (`self.MainCanvas`))
  (bind _returnvalue (`|CreateWidget` "/Game/BraveKnight/UI/WBP_MainCanvas.WBP_MainCanvas_C" (`GameplayStatics.GetPlayerController` 0)))
  (bind _output_get (set `self.MainCanvas` _returnvalue))
  (set `/Game/BraveKnight/UI/WBP_MainCanvas.Owner` self _output_get)
  (`UserWidget.AddToViewport` _output_get 0)
  (`|ExecutionSequence`
    (:`then_0`
      (bind _returnvalue_2 (`|CreateWidget` "/Game/BraveKnight/UI/WBP_HealthBar.WBP_HealthBar_C"))
      (bind _output_get_2 (set `self.HealthBar` _returnvalue_2))
      (set `/Game/BraveKnight/UI/WBP_HealthBar.OwnerRef` self _output_get_2)
      (`HorizontalBox.AddChildToHorizontalBox` (`/Game/BraveKnight/UI/WBP_MainCanvas.HealthContainer` _maincanvas) _output_get_2))
    (:`then_1`
      (bind _returnvalue_3 (`|CreateWidget` "/Game/BraveKnight/UI/WBP_StaminaBar.WBP_StaminaBar_C"))
      (bind _output_get_3 (set `self.StaminaBar` _returnvalue_3))
      (set `/Game/BraveKnight/UI/WBP_StaminaBar.OwnerRef` self _output_get_3)
      (`HorizontalBox.AddChildToHorizontalBox` (`/Game/BraveKnight/UI/WBP_MainCanvas.StaminaContainer` _maincanvas) _output_get_3))))

(event `self.ReceiveTick`
  (params (DeltaSeconds :type "Float (single-precision)"))
  (`parent.ReceiveTick` DeltaSeconds)
  (`KismetSystemLibrary.PrintString` (`KismetStringLibrary.Conv_DoubleToString` (`self.Stamina`)) true false (struct :`G` 0.66 :`B` 1.0 :`A` 1.0) 2.0 "1"))

(fn `UserConstructionScript`)