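; BP_Fires is a torch-style fire actor pairing a small temple fire particle effect with looping-style torch audio.
; On BeginPlay it activates the fire and configures the audio's sound, attenuation, concurrency and volume, playing from a random offset to desynchronize instances.
; FlareUp and FlareDown events drive the SpawnRateScale particle parameter to intensify or shut off the fire.
; The construction script provides an optional editor preview with its own spawn rate.
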(event `self.ReceiveBeginPlay`
  (bind _audio (`self.Audio`))
  ;[1 1 1] Init Fire
  (`ActorComponent.Activate` (`self.P_Temple_Fire_Small`) false)
  ;[1 1 1] Init Audio Component and Play Torch Sound
  (`self.InitializeAudioComponent` _audio)
  (`ActorComponent.Activate` _audio false)
  (`AudioComponent.Play` _audio (* (`KismetMathLibrary.RandomFloatInRange` 0.0 1.0) (`SoundBase.Duration` (`self.TorchSound`)))))

(event `self.ReceiveTick`
  (params (DeltaSeconds :type "Float (single-precision)")))

(event `FlareUp`
  (bind _p_temple_fire_small (`self.P_Temple_Fire_Small`))
  (`ActorComponent.Activate` _p_temple_fire_small false)
  ;[1 1 1] Careful with this, don't go over 2 or risk bad GPU!
  (`ParticleSystemComponent.SetFloatParameter` _p_temple_fire_small "SpawnRateScale" (`self.FlareUpSpawnRate`)))

(event `FlareDown`
  (bind _p_temple_fire_small (`self.P_Temple_Fire_Small`))
  ;[1 1 1] Turn Off Fire
  (`ParticleSystemComponent.SetFloatParameter` _p_temple_fire_small "SpawnRateScale" 0.0)
  (`ActorComponent.Deactivate` _p_temple_fire_small))

(fn `InitializeAudioComponent`
  (params (AudioComponentIn :type "AudioComponent Object Reference"))
  ;[1 1 1] Set Initial Values (Pass Through)
  (`AudioComponent.SetSound` AudioComponentIn (`self.TorchSound`))
  (set `AudioComponent.AttenuationSettings` (`self.TorchAttenuation`) AudioComponentIn)
  (set `AudioComponent.ConcurrencySet` (`|MakeSet` (`self.TorchConcurrency`)) AudioComponentIn)
  (`AudioComponent.SetVolumeMultiplier` AudioComponentIn (`self.BaseVolume`)))

(fn `UserConstructionScript`
  (`ActorComponent.SetAutoActivate` (`self.P_Temple_Fire_Small`) (`self.EnablePreviewFire`))
  (`ParticleSystemComponent.SetFloatParameter` (`self.P_Temple_Fire_Small`) "SpawnRateScale" (`self.PreviewSpawnRate`)))